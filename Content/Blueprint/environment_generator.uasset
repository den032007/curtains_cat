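; Environment generator actor that fills a row of randomly chosen background props along the Y axis when play begins.
; BeginPlay caches the actor's location, then loops, calling the random spawn event and stepping Y by a fixed increment.
; The spawn switch raises windows by a Z offset; two branches show no class, and the bed table branch is unreachable with the current random range.
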(event Custom|spawn_random_back
  (switch int (Math|Random|RandomInteger 3)
    (:0
      (Game|SpawnActorfromClass "/Game/Blueprint/chair.chair_C" (Math|Transform|MakeTransform (Math|Vector|MakeVector (Variables|Default|GetDefault%20X) (Variables|Default|Getchacngable_y) (Variables|Default|GetDefault%20Z)) "0,0.000000, 0" "1,1,1") "Undefined" 0 0))
    (:1
      (Game|SpawnActorfromClass "/Game/Blueprint/bed_table.bed_table_C" (Math|Transform|MakeTransform (Math|Vector|MakeVector (Variables|Default|GetDefault%20X) (Variables|Default|Getchacngable_y) (Variables|Default|GetDefault%20Z)) "0,0.000000, 0" "1,1,1") "Undefined" 0 0))
    (:2
      (Game|SpawnActorfromClass "/Game/Blueprint/window95.window95_C" (Math|Transform|MakeTransform (Math|Vector|MakeVector (Variables|Default|GetDefault%20X) (Variables|Default|Getchacngable_y) (+ (Variables|Default|GetDefault%20Z) (Variables|Default|Getwindow_offset))) "0,0.000000, 0" "1,1,1") "Undefined" 0 0))
    (:3
      (Game|SpawnActorfromClass "/Game/Blueprint/bed_table_3.bed_table_3_C" (Math|Transform|MakeTransform (Math|Vector|MakeVector (Variables|Default|GetDefault%20X) (Variables|Default|Getchacngable_y) (Variables|Default|GetDefault%20Z)) "0,0.000000, 0" "1,1,1") "Undefined" 0 0))))

(event EventBeginPlay
  (bind _returnvalue (Transformation|GetActorLocation))
  (Variables|Default|SetDefault%20X (.x _returnvalue))
  (bind _output_get (Variables|Default|SetDefault%20Y (.y _returnvalue)))
  (Variables|Default|Setchacngable_y _output_get)
  (Variables|Default|SetDefault%20Z (.z _returnvalue))
  (for _index (range 0 90)
    (CallFunction|SpawnRandomBack)
    (Variables|Default|Setchacngable_y (+ (Variables|Default|Getchacngable_y) (Variables|Default|Gety%20Increaser)))))

(event Collision|EventActorBeginOverlap
  (params (OtherActor :type Actor%20Object%20Reference)))

(event EventTick
  (params (DeltaSeconds :type Float%20%28single-precision%29)))

(fn ConstructionScript)