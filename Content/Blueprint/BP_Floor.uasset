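; BP_Floor is a floor actor with a kill box that ends the game when the cat pawn stays down on it.
; A BP_CatPawn entering the box starts a short one-shot timer.
; When it fires, the box rechecks its overlaps for any cat pawn, then marks the stored cat dead and calls GameOver on BP_PersistantGameMode.
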(event OnComponentBeginOverlap(KIllBox)
  (params (OverlappedComponent :type Primitive%20Component%20Object%20Reference) (OtherActor :type Actor%20Object%20Reference) (OtherComp :type Primitive%20Component%20Object%20Reference) (OtherBodyIndex :type Integer) (bFromSweep :type Boolean) (SweepResult :type Hit%20Result%20Structure%20%28by%20ref%29))
  (bind _asbp_cat_pawn (Utilities|Casting|CastToBP_CatPawn OtherActor))
  (Utilities|Time|SetTimerbyEvent (delegate Custom|TryKillCat) 1.5))

(event Custom|TryKillCat
  (if (> (Utilities|Array|Length (Collision|GetOverlappingActors (Variables|Default|GetKIllBox) "/Game/Blueprint/BP_CatPawn.BP_CatPawn_C" :!class /Script/Engine.PrimitiveComponent)) 0)
    (Variables|/Game/Blueprint/BP_CatPawn.BP_CatPawn_C|SetbIsDead (stale OnComponentBeginOverlap(KIllBox) _asbp_cat_pawn) true)
    (bind _asbp_persistant_game_mode (Utilities|Casting|CastToBP_PersistantGameMode (Game|GetGameMode)))
    (Default|GameOver _asbp_persistant_game_mode)))

(fn ConstructionScript)