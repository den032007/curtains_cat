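; Player camera manager Blueprint that adapts the default orthographic view width and aspect ratio to the viewport's shape.
; The construction script computes the viewport's aspect ratio once and stores it as the default.
; At or above a reference ratio, it scales the base ortho width proportionally to preserve vertical extent; narrower viewports keep the base width.
; The event graph contains only disabled placeholder events.
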(event EventBeginPlay)

(event Collision|EventActorBeginOverlap
  (params (OtherActor :type Actor%20Object%20Reference)))

(event EventTick
  (params (DeltaSeconds :type Float%20%28single-precision%29)))

(fn ConstructionScript
  (bind _returnvalue (Viewport|GetViewportSize))
  (bind (_x _y) (Math|Vector2D|BreakVector2D _returnvalue))
  (bind _output_get (Variables|Default|SetAspectRatio (/ _x _y)))
  (Variables|Default|SetDefaultAspectRatio _output_get)
  (if (>= (Variables|Default|GetAspectRatio) (Variables|Default|GetAspectRatioCheck))
    (Variables|Default|SetDefaultOrthoWidth (* (Variables|Default|GetOrdoWith) (/ (Variables|Default|GetAspectRatio) (Variables|Default|GetAspectRatioCheck))))
    (else
      (Variables|Default|SetDefaultOrthoWidth (Variables|Default|GetOrdoWith)))))