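; BP_CatPawn is the player's cat pawn, which jumps from hook to hook on left or right swap input.
; Swaps jump only while alive and allowed, enabling capsule physics and applying a velocity impulse; both sides share the identical impulse.
; OnHooked stops physics and re-arms jumping.
; The pawn registers itself with BP_CatPlayerController on BeginPlay and pins the camera to zero world rotation every tick.
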(event Custom|OnRightSwap
  (if (and (Variables|Default|GetbCanJump) (not (Variables|Default|GetbIsDead)))
    (CallFunction|PerformJumponRight)))

(event Custom|OnLeftSwap
  (if (and (Variables|Default|GetbCanJump) (not (Variables|Default|GetbIsDead)))
    (CallFunction|PerformJumponLeft)))

(event Custom|PerformJumpOnRight
  (bind _capsule (Variables|Default|GetCapsule))
  (Variables|Default|SetbCanJump false)
  (Physics|SetEnableGravity _capsule true)
  (Physics|SetSimulatePhysics _capsule true)
  (Physics|AddImpulse _capsule "0.000000,160.000000,900.000000" "None" true)
  (Utilities|FlowControl|Delay 1.0))

(event Custom|PerformJumpOnLeft
  (bind _capsule (Variables|Default|GetCapsule))
  (Variables|Default|SetbCanJump false)
  (Physics|SetEnableGravity _capsule true)
  (Physics|SetSimulatePhysics _capsule true)
  (Physics|AddImpulse _capsule "0.000000,160.000000,900.000000" "None" true)
  (Utilities|FlowControl|Delay 1.0))

(event Custom|OnHooked
  (Variables|Default|SetbCanJump true)
  (Physics|SetSimulatePhysics (Variables|Default|GetCapsule) false))

(event EventBeginPlay
  (bind _asbp_cat_player_controller (Utilities|Casting|CastToBP_CatPlayerController (Pawn|GetController)))
  (Variables|Default|SetPawnController _asbp_cat_player_controller)
  (Variables|/Game/Blueprint/BP_CatPlayerController.BP_CatPlayerController_C|SetControlledPawn _asbp_cat_player_controller self))

(event EventTick
  (params (DeltaSeconds :type Float%20%28single-precision%29))
  (Transformation|SetWorldRotation (Variables|Default|GetCamera) "0, 0, 0" false false))

(fn ConstructionScript)