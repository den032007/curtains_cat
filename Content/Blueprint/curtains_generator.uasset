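; Curtain generator actor that spawns a straight row of BP_Curtains actors when play begins.
; BeginPlay stores the generator's own location as the origin, then loops to spawn each curtain at the same X, Z and fixed rotation, stepping Y by YIncreaser after every spawn.
; The count is hard-coded in the loop, and the construction script is empty, so the row is built only at runtime.
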(event EventBeginPlay
  (bind _returnvalue (Transformation|GetActorLocation))
  (Variables|Default|SetdefaultX (.x _returnvalue))
  (bind _output_get (Variables|Default|SetdefaultY (.y _returnvalue)))
  (Variables|Default|Sety _output_get)
  (Variables|Default|SetdefaultZ (.z _returnvalue))
  (for _index (range 0 90)
    (Game|SpawnActorfromClass "/Game/Blueprint/BP_Curtains.BP_Curtains_C" (Math|Transform|MakeTransform (Math|Vector|MakeVector (Variables|Default|GetdefaultX) (Variables|Default|Gety) (Variables|Default|GetdefaultZ)) "0.000000,90.000000,0.000000" "1,1,1") "Undefined" 0 0)
    (Variables|Default|Sety (+ (Variables|Default|Gety) (Variables|Default|Gety_increaser)))))

(event Collision|EventActorBeginOverlap
  (params (OtherActor :type Actor%20Object%20Reference)))

(event EventTick
  (params (DeltaSeconds :type Float%20%28single-precision%29)))

(fn ConstructionScript)