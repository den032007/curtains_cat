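; Player controller for a cat game that handles touch swipes, keeps the score and creates the in-game HUD.
; A touch press stores the start location and arms per-tick swipe checks, built around distance-threshold comparisons on X or Y.
; A right swipe calls OnRightSwap on the controlled pawn, while a left swipe only prints a debug message.
; AddScorePoint accumulates the total and pushes it to the HUD.
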(event Custom|SwapRight
  (Development|PrintString "Swap on Right Handled")
  (Default|OnRightSwap (Variables|Default|GetControlledPawn)))

(event Custom|SwapLeft
  (Development|PrintString "Swap on Left Handled"))

(event Custom|AddScorePoint
  (params (ScorePointsToAdd :type Integer))
  (bind _output_get (Variables|Default|SetTotalScore (+ ScorePointsToAdd (Variables|Default|GetTotalScore))))
  (Default|UpdateTotalScore (stale EventBeginPlay _returnvalue) _output_get))

(event EventBeginPlay
  (bind _returnvalue (UserInterface|CreateWidget "/Game/Blueprint/InGameHUD.InGameHUD_C"))
  (UserInterface|Viewport|AddtoViewport _returnvalue 0))

(event EventTick
  (params (DeltaSeconds :type Float%20%28single-precision%29))
  (if (Variables|Default|GetbCanHandleSwap)
    (if (Utilities|BWasTouchSwaptoRight)
      (Variables|Default|SetbCanHandleSwap false)
      (CallFunction|SwapRight)
      (elif (Utilities|BWasTouchSwaptoLeft)
        (Variables|Default|SetbCanHandleSwap false)
        (CallFunction|SwapLeft)))))

(event Input|TouchEvents|InputTouch
  (params (Location :type Vector) (FingerIndex :type ETouchIndex%20Enum))
  (:Pressed
    (Variables|Default|SetbCanHandleSwap true)
    (Variables|Default|SetTouchStartLocation Location))
  (:Released
    (Variables|Default|SetbCanHandleSwap false)))

(fn ConstructionScript
  (Variables|Default|SetbShowMouseCursor true))